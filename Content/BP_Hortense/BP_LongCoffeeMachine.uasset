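; BP_LongCoffeeMachine is a coffee machine actor that serves one step of the player's coffee quest.
; When the third-person character overlaps its Collision in the required quest state, it passes that state to the character's CoffeeQuestManager.
; It then hands BrewCoffee to the character's BindEventToEndHold, presumably to run when a hold finishes.
; BrewCoffee spawns a BP_Coffee slightly above the SpawnPoint component.
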(event `self.Collision.OnComponentBeginOverlap`
  (params (OverlappedComponent :type "PrimitiveComponent Object Reference") (OtherActor :type "Actor Object Reference") (OtherComp :type "PrimitiveComponent Object Reference") (OtherBodyIndex :type Integer) (bFromSweep :type Boolean) (SweepResult :type "HitResult Structure (by ref)"))
  (bind _asbp_third_person_character (cast `/Game/ThirdPerson/Blueprints/BP_ThirdPersonCharacter` OtherActor))
  (bind _currentcoffeequeststate (`/Game/ThirdPerson/Blueprints/BP_ThirdPersonCharacter.CurrentCoffeeQuestState` _asbp_third_person_character))
  (if (`|EnumEquality` _currentcoffeequeststate "NewEnumerator1")
    (`/Game/ThirdPerson/Blueprints/BP_ThirdPersonCharacter.CoffeeQuestManager` _asbp_third_person_character _currentcoffeequeststate)
    (add `/Game/ThirdPerson/Blueprints/BP_ThirdPersonCharacter.EndHold` _asbp_third_person_character (delegate `BrewCoffee`))))

(event `BrewCoffee`
  (`|SpawnActorFromClass` "/Game/BP_Hortense/BP_Coffee.BP_Coffee_C" (`KismetMathLibrary.MakeTransform` (+ (`SceneComponent.K2_GetComponentLocation` (`self.SpawnPoint`)) (0.0 0.0 30.0))) "Undefined" "MultiplyWithRoot" null null))

(fn `UserConstructionScript`
  (`parent.UserConstructionScript`))