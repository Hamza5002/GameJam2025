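; Printer long-interactable that resolves the "Fix the printer" quest and awards its reward.
; BeginPlay sets the quest name, and Tick rebinds a handler to the third-person character's EndTouch event every frame.
; That handler searches BP_Quest's active quests for the hard-coded name, changes the matching entry's state and adds its reward to the player's score.
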(event `self.ReceiveBeginPlay`
  (`parent.ReceiveBeginPlay`)
  (set `self.NameOfQuest` "Fix the printer"))

(event `self.ReceiveTick`
  (params (DeltaSeconds :type "Float (single-precision)"))
  (`parent.ReceiveTick` DeltaSeconds)
  (bind _asbp_third_person_character (cast `/Game/ThirdPerson/Blueprints/BP_ThirdPersonCharacter` (`GameplayStatics.GetPlayerCharacter` 0)))
  (add `/Game/ThirdPerson/Blueprints/BP_ThirdPersonCharacter.EndTouch` _asbp_third_person_character (delegate `CustomEvent`)))

(event `CustomEvent`
  (bind _returnvalue (`GameplayStatics.GetActorOfClass` "/Game/ThirdPerson/Blueprints/BP_Quest.BP_Quest_C"))
  (bind _output_get (set `self.Quest` _returnvalue))
  (bind _activequests (`/Game/ThirdPerson/Blueprints/BP_Quest.ActiveQuests` _output_get))
  (for (_array_element _array_index) _activequests
    (if (== (break `/Game/ThirdPerson/Blueprints/ST_Quest` _array_element) "Fix the printer")
      (`KismetArrayLibrary.Array_Set` _activequests _array_index (make `/Game/ThirdPerson/Blueprints/ST_Quest` (break `/Game/ThirdPerson/Blueprints/ST_Quest` _array_element) (`.Icon_9_04E41BB74029662FF229EC928656F36E` (break `/Game/ThirdPerson/Blueprints/ST_Quest` _array_element)) (`.Temps_10_BC33AE564C487F56934656BF72819646` (break `/Game/ThirdPerson/Blueprints/ST_Quest` _array_element)) (`.Récompense_11_CD177A474A69A95EA8292789961EB17C` (break `/Game/ThirdPerson/Blueprints/ST_Quest` _array_element)) (`.WidgetRef_14_BA82D781437EBDEA82F3EAA606901CBA` (break `/Game/ThirdPerson/Blueprints/ST_Quest` _array_element)) "NewEnumerator2"))
      (bind _score (`/Game/ThirdPerson/Blueprints/BP_ThirdPersonCharacter.Score` (stale `self.ReceiveTick` _asbp_third_person_character)))
      (set `/Game/UI/WBP_SCORE.Score Points` (+ (`/Game/UI/WBP_SCORE.Score Points` _score) (`.Récompense_11_CD177A474A69A95EA8292789961EB17C` (break `/Game/ThirdPerson/Blueprints/ST_Quest` _array_element))) _score))))

(fn `UserConstructionScript`
  (`parent.UserConstructionScript`))