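; BP_PNJ is an NPC that patrols endlessly back and forth between two target actors, Target1 and Target2.
; It starts at Target1, then two timelines lerp its position and face it toward the destination, switching between walk and idle animations with a pause at each end.
; Capsule hits on the third-person player temporarily lower the player's max walk speed, with a DoOnce blocking retriggers until the speed is restored.
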(event `self.ReceiveBeginPlay`
  (bind (_returnvalue_location _returnvalue_rotation) (`KismetMathLibrary.BreakTransform` (`SceneComponent.K2_GetComponentToWorld` (`TargetPoint.ArrowComponent` (`self.Target 1`)))))
  (`self.K2_SetActorLocationAndRotation` _returnvalue_location _returnvalue_rotation)
  (`self.StartMove`))

(event `StartMove`
  (bind _returnvalue_location (`KismetMathLibrary.BreakTransform` (`SceneComponent.K2_GetComponentToWorld` (`Actor.RootComponent` (`self.Target2`)))))
  (bind _returnvalue (`SceneComponent.K2_GetComponentLocation` (`Actor.RootComponent` (`self.Target 1`))))
  (`SkeletalMeshComponent.PlayAnimation` (`self.Mesh`) "/Game/Characters/Mannequins/Animations/Quinn/MF_Walk_Fwd.MF_Walk_Fwd" true)
  (bind (_direction _newtrack_0) (`Timeline|Timeline` :!via `PlayFromStart`)
    (:`Update`
      (`self.K2_SetActorLocationAndRotation` (`KismetMathLibrary.VLerp` _returnvalue _returnvalue_location _newtrack_0) (`KismetMathLibrary.FindLookAtRotation` _returnvalue _returnvalue_location)))
    (:`Finished`
      (`SkeletalMeshComponent.PlayAnimation` (`self.Mesh`) "/Game/Characters/Mannequins/Animations/Quinn/MF_Idle.MF_Idle" true)
      (`KismetSystemLibrary.Delay` 3.0)
      (`self.EndMove`))))

(event `EndMove`
  (bind _returnvalue_location (`KismetMathLibrary.BreakTransform` (`SceneComponent.K2_GetComponentToWorld` (`Actor.RootComponent` (`self.Target2`)))))
  (bind _returnvalue (`SceneComponent.K2_GetComponentLocation` (`TargetPoint.ArrowComponent` (`self.Target 1`))))
  (`SkeletalMeshComponent.PlayAnimation` (`self.Mesh`) "/Game/Characters/Mannequins/Animations/Quinn/MF_Walk_Fwd.MF_Walk_Fwd" true)
  (bind (_direction _newtrack_0) (`Timeline|Timeline_0` :!via `PlayFromStart`)
    (:`Update`
      (`self.K2_SetActorLocationAndRotation` (`KismetMathLibrary.VLerp` _returnvalue_location _returnvalue _newtrack_0) (`KismetMathLibrary.FindLookAtRotation` _returnvalue_location _returnvalue)))
    (:`Finished`
      (`SkeletalMeshComponent.PlayAnimation` (`self.Mesh`) "/Game/Characters/Mannequins/Animations/Quinn/MF_Idle.MF_Idle" true)
      (`KismetSystemLibrary.Delay` 3.0)
      (`self.StartMove`))))

(event `self.CapsuleComponent.OnComponentHit`
  (params (HitComponent :type "PrimitiveComponent Object Reference") (OtherActor :type "Actor Object Reference") (OtherComp :type "PrimitiveComponent Object Reference") (NormalImpulse :type "Vector Structure") (Hit :type "HitResult Structure (by ref)"))
  (bind _asbp_third_person_character (cast `/Game/ThirdPerson/Blueprints/BP_ThirdPersonCharacter` OtherActor))
  (`KismetSystemLibrary.PrintString` "collision")
  (`/Engine/EditorBlueprintResources/StandardMacros.DoOnce` false :!label _label
    (:`Completed`
      (bind _charactermovement (`Character.CharacterMovement` _asbp_third_person_character))
      (set `CharacterMovementComponent.MaxWalkSpeed` 200.0 _charactermovement)
      (`KismetSystemLibrary.Delay` 5.0)
      (set `CharacterMovementComponent.MaxWalkSpeed` 500.0 _charactermovement)
      (goto _label :!via `Reset`))))

(fn `UserConstructionScript`)