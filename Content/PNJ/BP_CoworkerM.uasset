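; BP_CoworkerM is a coworker NPC that loops an idle animation and serves as the delivery target for the coffee quest.
; While NeedCoffee is set, a capsule hit from an interacting player holding BP_Coffee destroys the cup and clears the need.
; It then resets the player's RandomPNJ and reports through the player's CoffeeQuestManager.
; An unconnected graph that updates BP_Quest's active quests and score never runs.
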(event `self.ReceiveBeginPlay`
  (`SkeletalMeshComponent.PlayAnimation` (`self.Mesh`) "/Game/Characters/Mannequins/Animations/Manny/MM_Idle.MM_Idle" true)
  (bind _returnvalue (`GameplayStatics.GetActorOfClass` "/Game/ThirdPerson/Blueprints/BP_Quest.BP_Quest_C"))
  (set `self.Quest` _returnvalue))

(event `self.CapsuleComponent.OnComponentHit`
  (params (HitComponent :type "PrimitiveComponent Object Reference") (OtherActor :type "Actor Object Reference") (OtherComp :type "PrimitiveComponent Object Reference") (NormalImpulse :type "Vector Structure") (Hit :type "HitResult Structure (by ref)"))
  (if (`self.NeedCoffee`)
    (`KismetSystemLibrary.PrintString` "NeedCoffee" true true (struct :`R` 1.0 :`G` 0.14355 :`B` 0.203285 :`A` 1.0))
    (bind _asbp_third_person_character (cast `/Game/ThirdPerson/Blueprints/BP_ThirdPersonCharacter` OtherActor))
    (if (`/Game/ThirdPerson/Blueprints/BP_ThirdPersonCharacter.IsInteracting?` _asbp_third_person_character)
      (bind _heldobject (`/Game/ThirdPerson/Blueprints/BP_ThirdPersonCharacter.HeldObject` _asbp_third_person_character))
      (if (== (`GameplayStatics.GetObjectClass` _heldobject) "/Game/BP_Hortense/BP_Coffee.BP_Coffee_C")
        (`self.K2_DetachFromActor` _heldobject "KeepWorld" "KeepWorld" "KeepWorld")
        (`self.SetActorEnableCollision` _heldobject true)
        (set `/Game/ThirdPerson/Blueprints/BP_ThirdPersonCharacter.IsInteracting?` false _asbp_third_person_character)
        (`self.K2_DestroyActor` _heldobject)
        (set `/Game/ThirdPerson/Blueprints/BP_ThirdPersonCharacter.RandomPNJ` null _asbp_third_person_character)
        (`/Game/ThirdPerson/Blueprints/BP_ThirdPersonCharacter.CoffeeQuestManager` _asbp_third_person_character "NewEnumerator0")
        (set `self.NeedCoffee` false)))))

(fn `UserConstructionScript`)