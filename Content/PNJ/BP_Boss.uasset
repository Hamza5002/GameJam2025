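; BP_Boss is an idle-animated NPC that receives the coffee for the "Go get coffee" quest.
; When an interacting third-person character holding a BP_Coffee hits its capsule, it detaches and destroys the coffee and clears the interaction flag.
; It then finds BP_Quest in the level, updates the state of matching active quests by rewriting their struct, and adds their reward to the player's score.
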(event `self.ReceiveBeginPlay`
  (`SkeletalMeshComponent.PlayAnimation` (`self.Mesh`) "/Game/Characters/Mannequins/Animations/Manny/MM_Idle.MM_Idle" true)
  (bind _returnvalue (`GameplayStatics.GetActorOfClass` "/Game/ThirdPerson/Blueprints/BP_Quest.BP_Quest_C"))
  (set `self.Quest` _returnvalue))

(event `self.CapsuleComponent.OnComponentHit`
  (params (HitComponent :type "PrimitiveComponent Object Reference") (OtherActor :type "Actor Object Reference") (OtherComp :type "PrimitiveComponent Object Reference") (NormalImpulse :type "Vector Structure") (Hit :type "HitResult Structure (by ref)"))
  (bind _asbp_third_person_character (cast `/Game/ThirdPerson/Blueprints/BP_ThirdPersonCharacter` OtherActor))
  (if (`/Game/ThirdPerson/Blueprints/BP_ThirdPersonCharacter.IsInteracting?` _asbp_third_person_character)
    (bind _heldobject (`/Game/ThirdPerson/Blueprints/BP_ThirdPersonCharacter.HeldObject` _asbp_third_person_character))
    (if (== (`GameplayStatics.GetObjectClass` _heldobject) "/Game/BP_Hortense/BP_Coffee.BP_Coffee_C")
      (`self.K2_DetachFromActor` _heldobject "KeepWorld" "KeepWorld" "KeepWorld")
      (`self.SetActorEnableCollision` _heldobject true)
      (set `/Game/ThirdPerson/Blueprints/BP_ThirdPersonCharacter.IsInteracting?` false _asbp_third_person_character)
      (`self.K2_DestroyActor` _heldobject)
      (bind _returnvalue (`GameplayStatics.GetActorOfClass` "/Game/ThirdPerson/Blueprints/BP_Quest.BP_Quest_C"))
      (bind _output_get (set `self.Quest` _returnvalue))
      (bind _activequests (`/Game/ThirdPerson/Blueprints/BP_Quest.ActiveQuests` _output_get))
      (for (_array_element _array_index) _activequests
        (bind (_questtype _questname _icon _temps `_récompense` _widgetref) (break `/Game/ThirdPerson/Blueprints/ST_Quest` _array_element))
        (if (== _questname "Go get coffee")
          (`KismetArrayLibrary.Array_Set` _activequests _array_index (make `/Game/ThirdPerson/Blueprints/ST_Quest` _questtype _questname _icon _temps `_récompense` _widgetref "NewEnumerator2"))
          (bind _score (`/Game/ThirdPerson/Blueprints/BP_ThirdPersonCharacter.Score` _asbp_third_person_character))
          (set `/Game/UI/WBP_SCORE.Score Points` (+ (`/Game/UI/WBP_SCORE.Score Points` _score) `_récompense`) _score))))))

(fn `UserConstructionScript`)